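; BP_BaseKey is a collectible key that records on the collecting player's state that they hold a red or green key.
; OnCollect runs its logic only with authority and checks that the collecting avatar is valid.
; It switches on KeyType, casts the avatar controller's PlayerState to FinalPlayerState and sets the matching HasRedKey or HasGreenKey flag.
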(event `self.OnCollect`
  (params (CollectedAvatar :type "FinalAvatar Object Reference"))
  (bind (_asfinal_player_state _bsuccess) (cast `FinalPlayerState` (`Controller.PlayerState` (`Pawn.GetController` CollectedAvatar)) :!pure true))
  (`/Engine/EditorBlueprintResources/ActorMacros.Switch Has Authority`
    (:`Authority`
      (`/Engine/EditorBlueprintResources/StandardMacros.IsValid` CollectedAvatar
        (:`Is Valid`
          (switch `EFinalBaseKeyType` (`self.KeyType`)
            (:`RedKey`
              (if _bsuccess
                (set `FinalPlayerState.bHasRedKey` true _asfinal_player_state)))
            (:`GreenKey`
              (if _bsuccess
                (set `FinalPlayerState.bHasGreenKey` true _asfinal_player_state)))))))))

(fn `UserConstructionScript`)