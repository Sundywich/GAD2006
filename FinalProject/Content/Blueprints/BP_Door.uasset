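; A keyed door actor that slides upward when an interacting avatar holds the matching red or green key.
; The construction script colours the mesh by KeyType, and DoorInteract checks the key flags on the avatar's FinalPlayerState.
; A one-shot timeline per colour lerps from the current location each update, so movement accumulates rather than following fixed endpoints, then sets IsOpened when finished.
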(event `self.DoorInteract`
  (params (InteractingAvatar :type "FinalAvatar Object Reference"))
  (bind _returnvalue (`self.K2_GetActorLocation`))
  (bind _returnvalue_2 (`self.K2_GetActorLocation`))
  (bind _asfinal_player_state (cast `FinalPlayerState` (`Controller.PlayerState` (`Pawn.GetController` InteractingAvatar)) :!pure true))
  (`/Engine/EditorBlueprintResources/StandardMacros.IsValid` InteractingAvatar
    (:`Is Valid`
      (if (not (`self.bIsOpened`))
        (switch `EFinalBaseKeyType` (`self.KeyType`)
          (:`RedKey`
            (if (`FinalPlayerState.bHasRedKey` _asfinal_player_state)
              (`/Engine/EditorBlueprintResources/StandardMacros.DoOnce` false
                (:`Completed`
                  (bind (_direction _float) (`Timeline|DoorOpenedByRed`)
                    (:`Update`
                      (`self.K2_SetActorLocation` (`KismetMathLibrary.VLerp` _returnvalue_2 (+ _returnvalue_2 (0.0 0.0 399.0)) _float)))
                    (:`Finished`
                      (set `self.bIsOpened` true :!label _label)))))))
          (:`GreenKey`
            (if (`FinalPlayerState.bHasGreenKey` _asfinal_player_state)
              (`/Engine/EditorBlueprintResources/StandardMacros.DoOnce` false
                (:`Completed`
                  (bind (_direction_2 _float_2) (`Timeline|DoorOpenedByGreen`)
                    (:`Update`
                      (`self.K2_SetActorLocation` (`KismetMathLibrary.VLerp` _returnvalue (+ _returnvalue (0.0 0.0 399.0)) _float_2)))
                    (:`Finished`
                      (goto _label))))))))))))

(fn `UserConstructionScript`
  (bind _doormesh (`self.DoorMesh`))
  (switch `EFinalBaseKeyType` (`self.KeyType`)
    (:`RedKey`
      (`PrimitiveComponent.SetMaterial` _doormesh 0 "/AnimationSharing/AnimSharingRed.AnimSharingRed"))
    (:`GreenKey`
      (`PrimitiveComponent.SetMaterial` _doormesh 0 "/AnimationSharing/AnimSharingGreen.AnimSharingGreen"))))