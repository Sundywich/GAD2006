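; BP_GameState is the networked game state that handles match results and timer updates.
; On victory it tells each player's avatar whether it won or lost by player index, then shows a results widget.
; The message compares the winner's team with the local player's to show a loss or the winner's nickname, and restart removes it.
; Timer updates are forwarded through SendTimer to a dispatcher.
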(event `self.OnVictory`
  ;[1 1 1] Old OnVictory code
  (for _array_element (`self.PlayerArray`)
    (bind _asnet_player_state (cast `NetPlayerState` _array_element))
    (if (== (`self.WinningPlayer`) (`NetPlayerState.PlayerIndex` _asnet_player_state))
      (bind _asbp_net_avatar (cast `/Game/Blueprints/BP_NetAvatar` (`PlayerState.PawnPrivate` _asnet_player_state) :!pure true))
      (`/Game/Blueprints/BP_NetAvatar.OnPlayerWon` _asbp_net_avatar)
      (else
        (`/Game/Blueprints/BP_NetAvatar.OnPlayerLost` _asbp_net_avatar))))
  (`self.ShowResultMessage`))

(event `self.OnRestart`
  (`Widget.RemoveFromParent` (`self.MessageWidget`)))

(event `self.UpdateTimerDisplay`
  (params (Time :type "Float (single-precision)"))
  (`self.SendTimer` Time))

(event `SendTimer`
  (params (TimerTime :type "Float (double-precision)"))
  (`self.TimerDispatcher` TimerTime))

(fn `ShowResultMessage`
  (bind (_data_nickname _data_customizationdata _data_teamid) (break `SPlayerInfo` (`NetPlayerState.Data` (cast `NetPlayerState` (`Controller.PlayerState` (`GameplayStatics.GetPlayerController` 0)) :!pure true))))
  (bind _returnvalue (`self.GetPlayerStateByIndex` (`self.WinningPlayer`)))
  (bind (_data_nickname_2 _data_customizationdata_2 _data_teamid_2) (break `SPlayerInfo` (`NetPlayerState.Data` _returnvalue)))
  (bind _returnvalue_2 (`|CreateWidget` "/Game/Blueprints/UMG/W_GameResults.W_GameResults_C" null (select `bool` (`|EnumInequality` _data_teamid_2 _data_teamid) :`false` (`|FormatText` "{Name} WINSS!!" _data_nickname_2) :`true` "YOU LOST!!!!")))
  (set `self.MessageWidget` _returnvalue_2)
  (`UserWidget.AddToViewport` _returnvalue_2 0))

(fn `UserConstructionScript`)